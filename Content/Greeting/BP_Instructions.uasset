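; Greeting instructions Blueprint with five components, M1 to M5, that appear from the variable names to display a heading and subtext.
; On BeginPlay it creates a dynamic material instance on element 0 of each component.
; M1's instance is stored in TextRenderDMI, while M2 to M5 each overwrite SubtextRenderDMI, leaving only M5's referenced.
; No material parameters are set here, and the construction script is empty.
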(event `self.ReceiveBeginPlay`
  (`|ExecutionSequence`
    (:`then_0`
      (bind _returnvalue (`PrimitiveComponent.CreateDynamicMaterialInstance` (`self.m1`) 0 null))
      (set `self.TextRenderDMI` _returnvalue))
    (:`then_1`
      (bind _returnvalue_2 (`PrimitiveComponent.CreateDynamicMaterialInstance` (`self.m2`) 0 null))
      (set `self.SubtextRenderDMI` _returnvalue_2))
    (:`then_2`
      (bind _returnvalue_3 (`PrimitiveComponent.CreateDynamicMaterialInstance` (`self.m3`) 0 null))
      (set `self.SubtextRenderDMI` _returnvalue_3))
    (:`then_3`
      (bind _returnvalue_4 (`PrimitiveComponent.CreateDynamicMaterialInstance` (`self.m4`) 0 null))
      (set `self.SubtextRenderDMI` _returnvalue_4))
    (:`then_4`
      (bind _returnvalue_5 (`PrimitiveComponent.CreateDynamicMaterialInstance` (`self.m5`) 0 null))
      (set `self.SubtextRenderDMI` _returnvalue_5))))

(fn `UserConstructionScript`)